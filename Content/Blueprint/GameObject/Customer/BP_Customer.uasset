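; BP_Customer is the customer character Blueprint, handling animation, fading and purchase feedback.
; On BeginPlay it binds the destroy event and CrowdMovementComponent start and stop events, with handlers for looping walk and idle animations.
; Timelines drive Opacity on dynamic body and hair materials to fade the customer in on spawn and out before destroying the actor.
; A shop purchase spawns an effect actor and plays a buy sound with slight pitch variation.
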(event Custom|OnWalk
  (Components|Animation|PlayAnimation (Variables|Default|GetMainStaticMesh) "/Game/Assets/3D/Customer/CustomerWalk.CustomerWalk" true))

(event Custom|OnIdle
  (Components|Animation|PlayAnimation (Variables|Default|GetMainStaticMesh) "/Game/Assets/3D/Customer/CustomerIdle.CustomerIdle" true))

(event Custom|DoFadeOut
  (Utilities|IsValid (Variables|Default|GetDynMatBody)
    (:Is%20Valid
      (Utilities|IsValid (Variables|Default|GetDynMatHair)
        (:Is%20Valid
          (bind _opacity (Timeline|FadeOut PlayFromStart)
            (:Update
              (Rendering|Material|SetScalarParameterValue (Variables|Default|GetDynMatBody) "Opacity" _opacity :!class /Script/Engine.MaterialInstanceDynamic)
              (Rendering|Material|SetScalarParameterValue (Variables|Default|GetDynMatHair) "Opacity" _opacity :!class /Script/Engine.MaterialInstanceDynamic))
            (:Finished
              (Actor|DestroyActor))))))))

(event Custom|DoFadeIn
  (Utilities|IsValid (Variables|Default|GetDynMatBody)
    (:Is%20Valid
      (Utilities|IsValid (Variables|Default|GetDynMatHair)
        (:Is%20Valid
          (bind _opacity (Timeline|FadeIn PlayFromStart)
            (:Update
              (Rendering|Material|SetScalarParameterValue (Variables|Default|GetDynMatBody) "Opacity" _opacity :!class /Script/Engine.MaterialInstanceDynamic)
              (Rendering|Material|SetScalarParameterValue (Variables|Default|GetDynMatHair) "Opacity" _opacity :!class /Script/Engine.MaterialInstanceDynamic))))))))

(event EventBeginPlay
  (bind _mainstaticmesh (Variables|Default|GetMainStaticMesh))
  (bind _crowdmovementcomponent (Variables|Default|GetCrowdMovementComponent))
  ;[1 1 1] Connect events
  (EventDispatchers|BindEventtoOnCustomerDestroy (EventDispatchers|CreateEvent :!event Custom|DoFadeOut))
  (Utilities|IsValid _crowdmovementcomponent
    (:Is%20Valid
      (EventDispatchers|AssignOnMovingStarted _crowdmovementcomponent (EventDispatchers|CreateEvent :!event Custom|OnWalk))
      (EventDispatchers|AssignOnMovingStopped _crowdmovementcomponent (EventDispatchers|CreateEvent :!event Custom|OnIdle))
      ;[1 1 1] Set dynamic materials
      (bind _returnvalue (Rendering|Material|CreateDynamicMaterialInstance _mainstaticmesh 0 0 "None" :!class /Script/Engine.PrimitiveComponent))
      (Variables|Default|SetDynMatBody _returnvalue)
      (bind _returnvalue_2 (Rendering|Material|CreateDynamicMaterialInstance _mainstaticmesh 1 0 "None" :!class /Script/Engine.PrimitiveComponent))
      (Variables|Default|SetDynMatHair _returnvalue_2)
      (CallFunction|DoFadein))
    (:Is%20Not%20Valid
      (Development|PrintString "Navigation Movement Component is missing"))))

(event EventOnPurchasedfromShopBP
  (params (MoneySpent :type Integer))
  (Game|SpawnActorfromClass "/Game/Blueprint/GameObject/Effect/BP_CustomerPurchaseEffect.BP_CustomerPurchaseEffect_C" (Transformation|GetWorldTransform (Variables|Default|GetEffectSpawn)) "Undefined" "MultiplyWithRoot" 0 0)
  (Audio|PlaySound2D "/Game/Assets/Audio/SFX/Buy.Buy" 0.8 (Math|Random|RandomFloatinRange 0.98 1.02) 0.0 0 0))

(fn ConstructionScript)